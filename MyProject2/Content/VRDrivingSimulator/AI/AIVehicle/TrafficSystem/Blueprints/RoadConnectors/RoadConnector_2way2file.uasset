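; Road connector for the AI traffic system that joins a road piece to another connector, with two In and two Out lane nodes.
; Setup links each Out node crosswise to the target's In nodes when the connection changes, records it on the parent road by compass position, and calls the target's Setup back.
; It rebuilds debug arrows for the connection and node links, and PaintArrows labels each node with its display name.
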(event EventBeginPlay)

(event Collision|EventActorBeginOverlap
  (params (OtherActor :type Actor%20Object%20Reference)))

(event EventTick
  (params (DeltaSeconds :type Float%20%28single-precision%29)))

(fn ConstructionScript
  (|CallParentFunction))

(fn Setup
  (params (In :type Array%20of%20Fixed%20Street%20Node%20Object%20References) (Out :type Array%20of%20Fixed%20Street%20Node%20Object%20References) (ConnectTo :type Road%20Connector%202way%202file%20Object%20Reference) (RoadComponent :type Road%20Parent%20Object%20Reference))
  (bind _returnvalue (Transformation|GetActorLocation))
  (bind _array (Utilities|Array|MakeArray 0))
  (if (and (== (Utilities|Array|Length In) 2) (== (Utilities|Array|Length Out) 2))
    (Variables|Default|SetIn In)
    (Variables|Default|SetOut Out))
  (if (!= RoadComponent 0)
    (Variables|Default|SetRoadComponent RoadComponent))
  (Variables|Default|SetTemp (and (!= ConnectTo 0) (!= ConnectTo (Variables|Default|GetConnectTo))))
  ;[1 1 1] Paint Arrow
  (if (and (!= ConnectTo 0) (!= ConnectTo (Variables|Default|GetConnectTo)))
    (Variables|Default|SetConnectTo ConnectTo))
  ;;[1 1 1] Delete existing Arrowcomponents before being redrawn
  (for _array_element (Variables|Default|GetArrowComponents)
    (Components|DestroyComponent _array_element))
  (Utilities|IsValid (Variables|Default|GetConnectTo)
    (:Is%20Valid
      (bind _returnvalue_2 (AddComponent|AddArrowComponent true (Math|Transform|MakeTransform (+ _returnvalue "0, 0,135.000000") (Math|Rotator|FindLookatRotation _returnvalue (Transformation|GetActorLocation (Variables|Default|GetConnectTo))) (Math|Vector|MakeVector (.x (* (/ "1.000000,1.000000,1.000000" 8e+01) (Math|Vector|VectorLength (- _returnvalue (Transformation|GetActorLocation (Variables|Default|GetConnectTo)))))) 2.0 1.0))))
      (Rendering|SetVisibility _returnvalue_2 true false)
      (Class|ArrowComponent|SetArrowColorNew _returnvalue_2 "(R=0.927199,G=1.000000,B=0.980653,A=1.000000)")
      (Utilities|Array|Add (Variables|Default|GetArrowComponents) _returnvalue_2)
      (if (Variables|Default|GetTemp)
        (Variables|/Game/VRDrivingSimulator/AI/AIVehicle/TrafficSystem/Blueprints/FixedStreetNode.FixedStreetNode_C|SetNextNodes (Utilities|Array|Get(acopy) (Variables|Default|GetOut)) (Utilities|Array|MakeArray (Utilities|Struct|MakeNextNodeStruct (Utilities|Array|Get(acopy) (Variables|RoadConnector_2way2file_C|GetIn (Variables|Default|GetConnectTo)) 1) 1e+02)))
        (Variables|/Game/VRDrivingSimulator/AI/AIVehicle/TrafficSystem/Blueprints/FixedStreetNode.FixedStreetNode_C|SetNextNodes (Utilities|Array|Get(acopy) (Variables|Default|GetOut) 1) (Utilities|Array|MakeArray (Utilities|Struct|MakeNextNodeStruct (Utilities|Array|Get(acopy) (Variables|RoadConnector_2way2file_C|GetIn (Variables|Default|GetConnectTo))) 1e+02)))
        (CallFunction|PaintArrows (Variables|Default|GetOut))
        (switch Utilities|FlowControl|Switch|SwitchonPosition (Variables|Default|GetPosition)
          (:NewEnumerator0
            (bind _asroad_parent_t (Utilities|Casting|CastToRoadParent_T (Variables|Default|GetRoadComponent)))
            (Variables|/Game/VRDrivingSimulator/Finished_components/Roads/RoadParent_T.RoadParent_T_C|SetConnectToNorth _asroad_parent_t (Variables|Default|GetConnectTo)))
          (:NewEnumerator1
            (Variables|/Game/VRDrivingSimulator/Finished_components/Roads/RoadParent.RoadParent_C|SetConnectToEast (Variables|Default|GetRoadComponent) (Variables|Default|GetConnectTo)))
          (:NewEnumerator2
            (bind _asroad_parent_x (Utilities|Casting|CastToRoadParent_X (Variables|Default|GetRoadComponent)))
            (Variables|/Game/VRDrivingSimulator/Finished_components/Roads/RoadParent_X.RoadParent_X_C|SetConnectToSouth _asroad_parent_x (Variables|Default|GetConnectTo)))
          (:NewEnumerator3
            (Variables|/Game/VRDrivingSimulator/Finished_components/Roads/RoadParent.RoadParent_C|SetConnectToWest (Variables|Default|GetRoadComponent) (Variables|Default|GetConnectTo))))
        (CallFunction|Setup (Variables|Default|GetConnectTo) _array _array self)
        (else
          (CallFunction|PaintArrows (Variables|Default|GetOut)))))))

(fn PaintArrows
  (params (Nodes :type Array%20of%20Fixed%20Street%20Node%20Object%20References))
  (for _array_element Nodes
    ;[1 1 1] Check this nodes next nodes and create an arrow between them
    (for _array_element_2 (Variables|/Game/VRDrivingSimulator/AI/AIVehicle/TrafficSystem/Blueprints/FixedStreetNode.FixedStreetNode_C|GetNextNodes _array_element)
      (Utilities|IsValid (.NextNode (Utilities|Struct|BreakNextNodeStruct _array_element_2))
        (:Is%20Valid
          (bind _returnvalue (AddComponent|AddArrowComponent true (Math|Transform|MakeTransform (+ (Transformation|GetActorLocation _array_element) "0, 0,20.000000") (Math|Rotator|FindLookatRotation (Transformation|GetActorLocation _array_element) (Transformation|GetActorLocation (.NextNode (Utilities|Struct|BreakNextNodeStruct _array_element_2)))) (Math|Vector|MakeVector (.x (* (/ "1.000000,1.000000,1.000000" 8e+01) (Math|Vector|VectorLength (- (Transformation|GetActorLocation _array_element) (Transformation|GetActorLocation (.NextNode (Utilities|Struct|BreakNextNodeStruct _array_element_2))))))) 1e+01 1.0))))
          (Rendering|SetVisibility _returnvalue true false)
          (Class|ArrowComponent|SetArrowColorNew _returnvalue "(R=0.000000,G=1.000000,B=0.022493,A=1.000000)")
          (Utilities|Array|Add (Variables|Default|GetArrowComponents) _returnvalue))))
    ;[1 1 1] Set the TextRenderer Name to the DisplayName of this node
    (Rendering|Components|TextRender|SetText (Variables|/Game/VRDrivingSimulator/AI/AIVehicle/TrafficSystem/Blueprints/FixedStreetNode.FixedStreetNode_C|GetName _array_element) (Utilities|Text|ToText(String) (Utilities|GetDisplayName _array_element)))))