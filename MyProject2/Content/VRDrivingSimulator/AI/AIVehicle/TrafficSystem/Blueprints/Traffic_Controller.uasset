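; Traffic junction controller for the driving simulator's AI traffic, copied from TrafficLight_Controller, that cycles signal states on traffic nodes and lights.
; On BeginPlay the first lane starts green and any crossing second lane red.
; A self-rearming ChangeLanes timer advances both lanes together through Red, RedYellow, Green, Yellow, refreshing each node and light.
; Every phase currently lasts equally long; older per-lane timer chains remain unconnected.
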(event Custom|InitLights
  (bind _secondlanenodes (Variables|Default|GetSecondLaneNodes))
  ;[1 1 1] Copy of TrafficLight_Controller, change to work as wanted
  ;;[1 1 1] Init the Traffic lights. The first lane gets Green as Start and if there is a second lanes crossing the first one, we make them red for the start
  (for _array_element (Variables|Default|GetFirstLaneNodes)
    (Variables|/Game/VRDrivingSimulator/AI/AIVehicle/TrafficSystem/Blueprints/TrafficLight_Parent.TrafficLight_Parent_C|SetState _array_element "NewEnumerator3")
    (Default|StateUpdated _array_element))
  (for _array_element_2 (Variables|Default|GetFirstLaneLights)
    (Variables|/Game/VRDrivingSimulator/Blueprints/Signs/Others/Traffic_light_bso.Traffic_light_bso_C|SetState _array_element_2 "NewEnumerator3")
    (Default|UpdateTraficLights _array_element_2))
  (if (> (Utilities|Array|Length _secondlanenodes) 0)
    (for _array_element_3 _secondlanenodes
      (Variables|/Game/VRDrivingSimulator/AI/AIVehicle/TrafficSystem/Blueprints/TrafficLight_Parent.TrafficLight_Parent_C|SetState _array_element_3 "NewEnumerator0")
      (Default|StateUpdated _array_element_3))
    (for _array_element_4 (Variables|Default|GetSecondLaneLights)
      (Variables|/Game/VRDrivingSimulator/Blueprints/Signs/Others/Traffic_light_bso.Traffic_light_bso_C|SetState _array_element_4 "NewEnumerator0")
      (Default|UpdateTraficLights _array_element_4))
    (else
      (Variables|Default|SetbOneLane true))))

(event EventBeginPlay
  ;[1 1 1] Copy of TrafficLight_Controller, change to work as wanted
  ;;[1 1 1] When start playing, initialize lanes and start timer
  (CallFunction|InitLights)
  (Utilities|Time|SetTimerbyFunctionName 0 "ChangeLanes" 2.0))

(fn ConstructionScript)

(fn ChangeFirstLaneState
  ;[1 1 1] Using the Enum and a timer to change the Color and state based on the current color and state
  (for _array_element (Variables|Default|GetFirstLaneNodes)
    (switch Utilities|FlowControl|Switch|SwitchonTrafficLightSettingsEnum (Variables|/Game/VRDrivingSimulator/AI/AIVehicle/TrafficSystem/Blueprints/TrafficLight_Parent.TrafficLight_Parent_C|GetState _array_element)
      (:NewEnumerator0
        (Variables|/Game/VRDrivingSimulator/AI/AIVehicle/TrafficSystem/Blueprints/TrafficLight_Parent.TrafficLight_Parent_C|SetState _array_element "NewEnumerator1"))
      (:NewEnumerator1
        (Variables|/Game/VRDrivingSimulator/AI/AIVehicle/TrafficSystem/Blueprints/TrafficLight_Parent.TrafficLight_Parent_C|SetState _array_element "NewEnumerator3"))
      (:NewEnumerator2
        (Variables|/Game/VRDrivingSimulator/AI/AIVehicle/TrafficSystem/Blueprints/TrafficLight_Parent.TrafficLight_Parent_C|SetState _array_element "NewEnumerator0"))
      (:NewEnumerator3
        (Variables|/Game/VRDrivingSimulator/AI/AIVehicle/TrafficSystem/Blueprints/TrafficLight_Parent.TrafficLight_Parent_C|SetState _array_element "NewEnumerator2")))
    (Default|StateUpdated _array_element))
  (for _array_element_2 (Variables|Default|GetFirstLaneLights)
    (switch Utilities|FlowControl|Switch|SwitchonTrafficLightSettingsEnum (Variables|/Game/VRDrivingSimulator/Blueprints/Signs/Others/Traffic_light_bso.Traffic_light_bso_C|GetState _array_element_2)
      (:NewEnumerator0
        (Variables|/Game/VRDrivingSimulator/Blueprints/Signs/Others/Traffic_light_bso.Traffic_light_bso_C|SetState _array_element_2 "NewEnumerator1"))
      (:NewEnumerator1
        (Variables|/Game/VRDrivingSimulator/Blueprints/Signs/Others/Traffic_light_bso.Traffic_light_bso_C|SetState _array_element_2 "NewEnumerator3"))
      (:NewEnumerator2
        (Variables|/Game/VRDrivingSimulator/Blueprints/Signs/Others/Traffic_light_bso.Traffic_light_bso_C|SetState _array_element_2 "NewEnumerator0"))
      (:NewEnumerator3
        (Variables|/Game/VRDrivingSimulator/Blueprints/Signs/Others/Traffic_light_bso.Traffic_light_bso_C|SetState _array_element_2 "NewEnumerator2")))
    (Default|UpdateTraficLights _array_element_2)))

(fn ChangeSecondLandState
  ;[1 1 1] Similar to the First Lane Changing
  (for _array_element (Variables|Default|GetSecondLaneNodes)
    (switch Utilities|FlowControl|Switch|SwitchonTrafficLightSettingsEnum (Variables|/Game/VRDrivingSimulator/AI/AIVehicle/TrafficSystem/Blueprints/TrafficLight_Parent.TrafficLight_Parent_C|GetState _array_element)
      (:NewEnumerator0
        (Variables|/Game/VRDrivingSimulator/AI/AIVehicle/TrafficSystem/Blueprints/TrafficLight_Parent.TrafficLight_Parent_C|SetState _array_element "NewEnumerator1"))
      (:NewEnumerator1
        (Variables|/Game/VRDrivingSimulator/AI/AIVehicle/TrafficSystem/Blueprints/TrafficLight_Parent.TrafficLight_Parent_C|SetState _array_element "NewEnumerator3"))
      (:NewEnumerator2
        (Variables|/Game/VRDrivingSimulator/AI/AIVehicle/TrafficSystem/Blueprints/TrafficLight_Parent.TrafficLight_Parent_C|SetState _array_element "NewEnumerator0"))
      (:NewEnumerator3
        (Variables|/Game/VRDrivingSimulator/AI/AIVehicle/TrafficSystem/Blueprints/TrafficLight_Parent.TrafficLight_Parent_C|SetState _array_element "NewEnumerator2")))
    (Default|StateUpdated _array_element))
  (for _array_element_2 (Variables|Default|GetSecondLaneLights)
    (switch Utilities|FlowControl|Switch|SwitchonTrafficLightSettingsEnum (Variables|/Game/VRDrivingSimulator/Blueprints/Signs/Others/Traffic_light_bso.Traffic_light_bso_C|GetState _array_element_2)
      (:NewEnumerator0
        (Variables|/Game/VRDrivingSimulator/Blueprints/Signs/Others/Traffic_light_bso.Traffic_light_bso_C|SetState _array_element_2 "NewEnumerator1"))
      (:NewEnumerator1
        (Variables|/Game/VRDrivingSimulator/Blueprints/Signs/Others/Traffic_light_bso.Traffic_light_bso_C|SetState _array_element_2 "NewEnumerator3"))
      (:NewEnumerator2
        (Variables|/Game/VRDrivingSimulator/Blueprints/Signs/Others/Traffic_light_bso.Traffic_light_bso_C|SetState _array_element_2 "NewEnumerator0"))
      (:NewEnumerator3
        (Variables|/Game/VRDrivingSimulator/Blueprints/Signs/Others/Traffic_light_bso.Traffic_light_bso_C|SetState _array_element_2 "NewEnumerator2")))
    (Default|UpdateTraficLights _array_element_2)))

(fn ChangeLanes
  ;[1 1 1] The flow for the controller. Change both lanes, wait the correct time and repeat
  (CallFunction|ChangeFirstLaneState)
  (CallFunction|ChangeSecondLandState)
  (switch Utilities|FlowControl|Switch|SwitchonTrafficLightSettingsEnum (Variables|/Game/VRDrivingSimulator/AI/AIVehicle/TrafficSystem/Blueprints/TrafficLight_Parent.TrafficLight_Parent_C|GetState (Utilities|Array|Get(acopy) (Variables|Default|GetFirstLaneNodes)))
    (:NewEnumerator0
      (Utilities|Time|SetTimerbyFunctionName 0 "ChangeLanes" 2.0))
    (:NewEnumerator1
      (Utilities|Time|SetTimerbyFunctionName 0 "ChangeLanes" 2.0))
    (:NewEnumerator2
      (Utilities|Time|SetTimerbyFunctionName 0 "ChangeLanes" 2.0))
    (:NewEnumerator3
      (Utilities|Time|SetTimerbyFunctionName 0 "ChangeLanes" 2.0))))