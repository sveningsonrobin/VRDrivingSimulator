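; AI car event node for the VR driving simulator's traffic system that holds a Red or Green state.
; On BeginPlay it copies the configured StartingState into State.
; SetStateRed, SetStateGreen and SetStateToggle change that state at runtime.
; Every change, including the initial one, calls StateUpdated, whose body is not defined in this graph.
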(event EventBeginPlay
  (switch Utilities|FlowControl|Switch|SwitchonEventNodeState (Variables|Default|GetStartingState)
    (:NewEnumerator0
      (Variables|Default|SetState "NewEnumerator0"))
    (:NewEnumerator1
      (Variables|Default|SetState "NewEnumerator3")))
  (CallFunction|StateUpdated))

(event EventActorBeginOverlap
  (params (OtherActor :type Actor%20Object%20Reference)))

(event EventTick
  (params (DeltaSeconds :type Float%20%28single-precision%29)))

(fn ConstructionScript
  (|CallParentFunction))

(fn SetStateRed
  (Variables|Default|SetState "NewEnumerator0")
  (CallFunction|StateUpdated))

(fn SetStateGreen
  (Variables|Default|SetState "NewEnumerator3")
  (CallFunction|StateUpdated))

(fn SetStateToggle
  (switch Utilities|FlowControl|Switch|SwitchonTrafficLightSettingsEnum (Variables|Default|GetState)
    (:NewEnumerator0
      (Variables|Default|SetState "NewEnumerator3"))
    (:NewEnumerator3
      (Variables|Default|SetState "NewEnumerator0")))
  (CallFunction|StateUpdated))