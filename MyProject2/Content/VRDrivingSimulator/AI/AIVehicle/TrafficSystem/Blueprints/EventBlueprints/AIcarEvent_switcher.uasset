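; AI traffic event actor that redirects AI cars to another path node when its trigger box is overlapped.
; On overlap, optionally filtered to a specific TriggerActor, it gets the overlapping Car_parent's AIcarCon controller and sets SwitchToNode as its target.
; The construction script draws a distance-scaled arrow toward SwitchToNode and labels the actor with its display name.
; SetStateRed is an empty stub.
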(event OnComponentBeginOverlap(Box)
  (params (OtherActor :type Actor%20Object%20Reference) (OtherComp :type Primitive%20Component%20Object%20Reference) (OtherBodyIndex :type Integer) (bFromSweep :type Boolean) (SweepResult :type Hit%20Result%20Structure%20%28by%20ref%29))
  (if (== (Variables|Default|GetTriggerActor) 0)
    (bind _ascar_parent (Utilities|Casting|CastToCar_parent OtherActor :!label _label))
    (bind _returnvalue (AI|GetAIController _ascar_parent))
    (bind _asaicar_con (Utilities|Casting|CastToAIcarCon _returnvalue))
    (Default|SetTargetNode _asaicar_con (Variables|Default|GetSwitchToNode))
    (elif (== OtherActor (Variables|Default|GetTriggerActor)) ; true = actor triggered the triggerbox
      (goto _label))))

(fn ConstructionScript
  (bind _returnvalue (Transformation|GetActorLocation))
  (bind _switchtonode (Variables|Default|GetSwitchToNode))
  (bind _returnvalue_2 (Transformation|GetActorLocation _switchtonode))
  (Utilities|IsValid _switchtonode
    (:Is%20Valid
      (bind _returnvalue_3 (AddComponent|AddArrowComponent true (Math|Transform|MakeTransform (+ _returnvalue "0, 0,20.000000") (Math|Rotator|FindLookatRotation _returnvalue _returnvalue_2) (Math|Vector|MakeVector (.x (* (/ "1.000000,1.000000,1.000000" 8e+01) (Math|Vector|VectorLength (- (Transformation|GetActorLocation) _returnvalue_2)))) 3.0 1.0))))
      (Rendering|SetVisibility _returnvalue_3 true false)
      (Class|ArrowComponent|SetArrowColorNew _returnvalue_3 "(R=1.000000,G=0.776667,B=0.000000,A=1.000000)")
      ;[1 1 1] Set the TextRenderer Name to the DisplayName of this node
      (Rendering|Components|TextRender|SetText (Variables|Default|GetName) (Utilities|Text|ToText(String) (Utilities|GetDisplayName self))))))

(fn SetStateRed
  (params (State :type TrafficLightSettingsEnum%20Enum)))