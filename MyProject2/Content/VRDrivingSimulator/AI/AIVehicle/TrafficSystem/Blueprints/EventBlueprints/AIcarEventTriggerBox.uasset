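; Trigger box for the AI traffic system that switches linked AI car event nodes to red when its assigned TriggerActor vehicle enters.
; On overlap, it sets a timer on each SetRed node to call SetStateRed after that entry's delay.
; The construction script draws stretched red, green and amber arrows to SetRed, SetGreen and Toggle nodes and labels the box with its name.
; SetGreen and Toggle have no runtime logic; the local SetStateRed is empty.
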(event EventBeginPlay)

(event EventActorBeginOverlap
  (params (OtherActor :type Actor%20Object%20Reference))
  (bind _aswheeled_vehicle (Utilities|Casting|CastToWheeledVehicle OtherActor))
  (if (== _aswheeled_vehicle (Variables|Default|GetTriggerActor)) ; true = actor triggered the triggerbox
    (Utilities|FlowControl|Sequence
      (:then_0
        (for _array_element (Variables|Default|GetSetRed)
          (Utilities|Time|SetTimerbyFunctionName (.AIcarEventNode (Utilities|Struct|BreakAIcarEventNodeDelayStruct _array_element)) "SetStateRed" (.DelayBeforeActivation (Utilities|Struct|BreakAIcarEventNodeDelayStruct _array_element))))))))

(event EventTick
  (params (DeltaSeconds :type Float%20%28single-precision%29)))

(fn ConstructionScript
  (bind _returnvalue (Transformation|GetActorLocation))
  (bind _returnvalue_2 (Transformation|GetActorLocation))
  (bind _returnvalue_3 (Transformation|GetActorLocation))
  ;[1 1 1] Create arrow to SetRed Nodes
  (for _array_element (Variables|Default|GetSetRed)
    (Utilities|IsValid (.AIcarEventNode (Utilities|Struct|BreakAIcarEventNodeDelayStruct _array_element))
      (:Is%20Valid
        (bind _returnvalue_4 (AddComponent|AddArrowComponent true (Math|Transform|MakeTransform (+ _returnvalue_2 "0, 0,20.000000") (Math|Rotator|FindLookatRotation _returnvalue_2 (Transformation|GetActorLocation (.AIcarEventNode (Utilities|Struct|BreakAIcarEventNodeDelayStruct _array_element)))) (Math|Vector|MakeVector (.x (* (/ "1.000000,1.000000,1.000000" 8e+01) (Math|Vector|VectorLength (- (Transformation|GetActorLocation) (Transformation|GetActorLocation (.AIcarEventNode (Utilities|Struct|BreakAIcarEventNodeDelayStruct _array_element))))))) 3.0 1.0))))
        (Rendering|SetVisibility _returnvalue_4 true false)
        (Class|ArrowComponent|SetArrowColorNew _returnvalue_4 "(R=1.000000,G=0.009362,B=0.000000,A=1.000000)"))))
  ;[1 1 1] Create arrow to SetGreen Nodes
  (for _array_element_2 (Variables|Default|GetSetGreen)
    (Utilities|IsValid (.AIcarEventNode (Utilities|Struct|BreakAIcarEventNodeDelayStruct _array_element_2))
      (:Is%20Valid
        (bind _returnvalue_5 (AddComponent|AddArrowComponent true (Math|Transform|MakeTransform (+ _returnvalue_3 "0, 0,20.000000") (Math|Rotator|FindLookatRotation _returnvalue_3 (Transformation|GetActorLocation (.AIcarEventNode (Utilities|Struct|BreakAIcarEventNodeDelayStruct _array_element_2)))) (Math|Vector|MakeVector (.x (* (/ "1.000000,1.000000,1.000000" 8e+01) (Math|Vector|VectorLength (- (Transformation|GetActorLocation) (Transformation|GetActorLocation (.AIcarEventNode (Utilities|Struct|BreakAIcarEventNodeDelayStruct _array_element_2))))))) 3.0 1.0))))
        (Rendering|SetVisibility _returnvalue_5 true false)
        (Class|ArrowComponent|SetArrowColorNew _returnvalue_5 "(R=0.000000,G=1.000000,B=0.003621,A=1.000000)"))))
  ;[1 1 1] Create arrow to SetGreen Nodes
  (for _array_element_3 (Variables|Default|GetToggle)
    (Utilities|IsValid (.AIcarEventNode (Utilities|Struct|BreakAIcarEventNodeDelayStruct _array_element_3))
      (:Is%20Valid
        (bind _returnvalue_6 (AddComponent|AddArrowComponent true (Math|Transform|MakeTransform (+ _returnvalue "0, 0,20.000000") (Math|Rotator|FindLookatRotation _returnvalue (Transformation|GetActorLocation (.AIcarEventNode (Utilities|Struct|BreakAIcarEventNodeDelayStruct _array_element_3)))) (Math|Vector|MakeVector (.x (* (/ "1.000000,1.000000,1.000000" 8e+01) (Math|Vector|VectorLength (- (Transformation|GetActorLocation) (Transformation|GetActorLocation (.AIcarEventNode (Utilities|Struct|BreakAIcarEventNodeDelayStruct _array_element_3))))))) 3.0 1.0))))
        (Rendering|SetVisibility _returnvalue_6 true false)
        (Class|ArrowComponent|SetArrowColorNew _returnvalue_6 "(R=1.000000,G=0.674767,B=0.000000,A=1.000000)"))))
  ;[1 1 1] Set the TextRenderer Name to the DisplayName of this node
  (Rendering|Components|TextRender|SetText (Variables|Default|GetName) (Utilities|Text|ToText(String) (Utilities|GetDisplayName self))))

(fn SetStateRed
  (params (State :type TrafficLightSettingsEnum%20Enum)))