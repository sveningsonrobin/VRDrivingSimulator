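; Traffic light street node for the AI vehicle traffic system, showing its current signal state through red, yellow and green components.
; StateUpdated switches on the State enum to toggle light visibility, with debug prints for red and green.
; The green-state loop over AcceptRadius overlaps, meant to restart cars, and SwitchTrafficLight are empty stubs.
; A work-in-progress event spawns an offset FixedStreetNode and appends it to NextNodesOld.
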(event Custom|TL_CreateNewNextNode
  ;[1 0 0] HIGHLY WIP
  (bind _returnvalue (Game|SpawnActorfromClass "/Game/VRDrivingSimulator/AI/AIVehicle/TrafficSystem/Blueprints/FixedStreetNode.FixedStreetNode_C" (Math|Transform|MakeTransform (+ (Transformation|GetActorLocation) "200.000000, 0, 0") "0, 0, 0" "1,1,1") "AdjustIfPossibleButDontSpawnIfColliding" 0 0))
  (Utilities|Array|Add (Variables|Default|GetNextNodesOld) _returnvalue))

(event Custom|StateUpdated
  ;[1 1 1] This gets called once the Enum State is updated. Then we just active or deactivate (visibilty) the blocks
  (switch Utilities|FlowControl|Switch|SwitchonTrafficLightSettingsEnum (Variables|Default|GetState)
    (:NewEnumerator0
      (Rendering|SetVisibility (Variables|Default|GetRed) true false)
      (Rendering|SetVisibility (Variables|Default|GetYellow) false false)
      (Rendering|SetVisibility (Variables|Default|GetGreen) false false)
      ;[0.008735 1 0] Comment
      (Development|PrintString "red"))
    (:NewEnumerator1
      (Rendering|SetVisibility (Variables|Default|GetRed) true false)
      (Rendering|SetVisibility (Variables|Default|GetYellow) true false)
      (Rendering|SetVisibility (Variables|Default|GetGreen) false false))
    (:NewEnumerator2
      (Rendering|SetVisibility (Variables|Default|GetRed) false false)
      (Rendering|SetVisibility (Variables|Default|GetYellow) true false)
      (Rendering|SetVisibility (Variables|Default|GetGreen) false false))
    (:NewEnumerator3
      (Utilities|FlowControl|Sequence
        (:then_0
          (Rendering|SetVisibility (Variables|Default|GetRed) false false)
          (Rendering|SetVisibility (Variables|Default|GetYellow) false false)
          (Rendering|SetVisibility (Variables|Default|GetGreen) true false)
          (Development|PrintString "green"))
        (:then_1
          ;[1 0 0.09028] tell cars to start moving when we are green again. not used atm
          (for _array_element (Collision|GetOverlappingActors (Variables|Default|GetAcceptRadius) 0 :!class /Script/Engine.PrimitiveComponent)
            _))))))

(event EventBeginPlay)

(event Collision|EventActorBeginOverlap
  (params (OtherActor :type Actor%20Object%20Reference)))

(event EventTick
  (params (DeltaSeconds :type Float%20%28single-precision%29))
  (|CallParentFunction 0.0))

(fn ConstructionScript
  (|CallParentFunction))

(fn SwitchTrafficLight
  ;[1 1 1] Nothing here yet
)