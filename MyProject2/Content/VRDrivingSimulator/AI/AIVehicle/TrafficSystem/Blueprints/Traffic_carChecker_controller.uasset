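; Traffic controller that switches traffic light street nodes according to vehicle presence in their linked car check boxes.
; On BeginPlay it sets every node in ControlledActors to a default state and registers itself with each entry's boxes.
; A box entry switches the nodes linked to that box to another state.
; On exit, a node reverts only once none of its boxes overlaps a WheeledVehicle.
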(event EventBeginPlay
  (for _array_element (Variables|Default|GetControlledActors)
    (Variables|/Game/VRDrivingSimulator/AI/AIVehicle/TrafficSystem/Blueprints/TrafficLight_Parent.TrafficLight_Parent_C|SetState (.TrafficLightStreetNode (Utilities|Struct|BreakCarCheck_TrafficLight_Link _array_element)) "NewEnumerator3")
    (Default|StateUpdated (.TrafficLightStreetNode (Utilities|Struct|BreakCarCheck_TrafficLight_Link _array_element)))
    (for _array_element_2 (.CarCheckBoxes (Utilities|Struct|BreakCarCheck_TrafficLight_Link _array_element))
      (Default|SetController _array_element_2 self))))

(fn ConstructionScript)

(fn CarEnteredBox
  (params (Box :type Car%20Checker%20Object%20Reference))
  (for _array_element (Variables|Default|GetControlledActors)
    (if (Utilities|Array|ContainsItem (.CarCheckBoxes (Utilities|Struct|BreakCarCheck_TrafficLight_Link _array_element)) Box)
      (Variables|/Game/VRDrivingSimulator/AI/AIVehicle/TrafficSystem/Blueprints/TrafficLight_Parent.TrafficLight_Parent_C|SetState (.TrafficLightStreetNode (Utilities|Struct|BreakCarCheck_TrafficLight_Link _array_element)) "NewEnumerator0")
      (Default|StateUpdated (.TrafficLightStreetNode (Utilities|Struct|BreakCarCheck_TrafficLight_Link _array_element))))))

(fn CarLeftBox
  (params (Box :type Car%20Checker%20Object%20Reference))
  (LocalVariables|SetNoOverlapping true)
  (bind _array_element (Utilities|Array|ForEachLoopwithBreak (Variables|Default|GetControlledActors))
    (:LoopBody
      (if (Utilities|Array|ContainsItem (.CarCheckBoxes (Utilities|Struct|BreakCarCheck_TrafficLight_Link _array_element)) Box)
        (bind _array_element_2 (Utilities|Array|ForEachLoopwithBreak (.CarCheckBoxes (Utilities|Struct|BreakCarCheck_TrafficLight_Link _array_element)) :!label _label)
          (:LoopBody
            (if (> (Utilities|Array|Length (Collision|GetOverlappingActors (Variables|/Game/VRDrivingSimulator/AI/AIVehicle/TrafficSystem/Blueprints/CarChecker.CarChecker_C|GetBox _array_element_2) "/Script/Engine.WheeledVehicle" :!class /Script/Engine.PrimitiveComponent)) 0)
              (LocalVariables|SetNoOverlapping false)
              (goto _label Break)))
          (:Completed
            (if (LocalVariables|GetNoOverlapping)
              (Variables|/Game/VRDrivingSimulator/AI/AIVehicle/TrafficSystem/Blueprints/TrafficLight_Parent.TrafficLight_Parent_C|SetState (.TrafficLightStreetNode (Utilities|Struct|BreakCarCheck_TrafficLight_Link _array_element)) "NewEnumerator3")
              (Default|StateUpdated (.TrafficLightStreetNode (Utilities|Struct|BreakCarCheck_TrafficLight_Link _array_element)))
              (else
                (LocalVariables|SetNoOverlapping true)))))))))