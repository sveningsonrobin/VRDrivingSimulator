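; FixedStreetNode is a waypoint actor in the AI vehicle traffic system, linked to successors through its NextNodes array.
; When an AI car overlaps its AcceptRadius, the node calls CallMoveCompleted on that car's controller if it is the current target.
; The construction script draws scaled green arrows toward each valid next node, labels the node and applies the inactive material.
; An unfinished editor event spawns an offset node into NextNodesOld.
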(event OnComponentBeginOverlap(AcceptRadius)
  (params (OtherActor :type Actor%20Object%20Reference) (OtherComp :type Primitive%20Component%20Object%20Reference) (OtherBodyIndex :type Integer) (bFromSweep :type Boolean) (SweepResult :type Hit%20Result%20Structure%20%28by%20ref%29))
  ;[1 1 1] When a Car overlaps this node, and this node is the current active node of the car, update the current node to the next one
  (bind _asaicar_vehicle (Utilities|Casting|CastToAIcarVehicle OtherActor))
  (bind _returnvalue (AI|GetAIController _asaicar_vehicle))
  (bind _asaicar_con (Utilities|Casting|CastToAIcarCon _returnvalue))
  (bind _streetnode (Default|GetTargetNode _asaicar_con))
  (if (== _streetnode self)
    (Default|CallMoveCompleted _asaicar_con)))

(event Custom|CreateNewNextNode
  ;[1 0 0] WIP | Test Button to spawn nodes from simple Buttonpress in Editor
  (bind _returnvalue (Game|SpawnActorfromClass "FixedStreetNode_C" (Math|Transform|MakeTransform (+ (Transformation|GetActorLocation) "200.000000, 0, 0") "0, 0, 0" "1,1,1") "AdjustIfPossibleButDontSpawnIfColliding" 0 0))
  (Utilities|Array|Add (Variables|Default|GetNextNodesOld) _returnvalue))

(fn ConstructionScript
  (bind _returnvalue (Transformation|GetActorLocation))
  ;[1 1 1] Check this nodes next nodes and create an arrow between them
  (for _array_element (Variables|Default|GetNextNodes)
    (Utilities|IsValid (.NextNode (Utilities|Struct|BreakNextNodeStruct _array_element))
      (:Is%20Valid
        (Utilities|FlowControl|Sequence
          (:then_0
            (bind _returnvalue_2 (AddComponent|AddArrowComponent true (Math|Transform|MakeTransform (+ _returnvalue "0, 0,20.000000") (Math|Rotator|FindLookatRotation _returnvalue (Transformation|GetActorLocation (.NextNode (Utilities|Struct|BreakNextNodeStruct _array_element)))) (Math|Vector|MakeVector (.x (* (/ "1.000000,1.000000,1.000000" 8e+01) (Math|Vector|VectorLength (- (Transformation|GetActorLocation) (Transformation|GetActorLocation (.NextNode (Utilities|Struct|BreakNextNodeStruct _array_element))))))) 1e+01 1.0))))
            (Rendering|SetVisibility _returnvalue_2 true false)
            (Class|ArrowComponent|SetArrowColorNew _returnvalue_2 "(R=0.000000,G=1.000000,B=0.022493,A=1.000000)"))))
      (:Is%20Not%20Valid
        (if (Variables|Default|GetRefreshConstructionScript)
          _))))
  ;[1 1 1] Set the TextRenderer Name to the DisplayName of this node
  (Rendering|Components|TextRender|SetText (Variables|Default|GetName) (Utilities|Text|ToText(String) (Utilities|GetDisplayName self)))
  ;[1 1 1] Set the Material of the Sphere to inactive at the beginning
  (Rendering|Material|SetMaterial (Variables|Default|GetAcceptSphere) 0 (Variables|Default|GetInactiveMat)))