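; CarChecker is a traffic system trigger that detects wheeled vehicles entering and leaving its Box component.
; Overlap events cast the other actor to WheeledVehicle and report CarEnteredBox or CarLeftBox to a CarCheckerController, passing itself as the source.
; The controller reference is injected through SetController, and the checker leaves any response to that controller.
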(event OnComponentBeginOverlap(Box)
  (params (OtherActor :type Actor%20Object%20Reference) (OtherComp :type Primitive%20Component%20Object%20Reference) (OtherBodyIndex :type Integer) (bFromSweep :type Boolean) (SweepResult :type Hit%20Result%20Structure%20%28by%20ref%29))
  (Utilities|Casting|CastToWheeledVehicle OtherActor)
  (Default|CarEnteredBox (Variables|Default|GetcarChecker_controller) self))

(event OnComponentEndOverlap(Box)
  (params (OtherActor :type Actor%20Object%20Reference) (OtherComp :type Primitive%20Component%20Object%20Reference) (OtherBodyIndex :type Integer))
  (Utilities|Casting|CastToWheeledVehicle OtherActor)
  (Default|CarLeftBox (Variables|Default|GetcarChecker_controller) self))

(event Custom|SetController
  (params (CarCheckerController :type Traffic%20Car%20Checker%20Controller%20Object%20Reference))
  (Variables|Default|SetcarChecker_controller CarCheckerController))

(event EventBeginPlay)

(event EventActorBeginOverlap
  (params (OtherActor :type Actor%20Object%20Reference)))

(event EventTick
  (params (DeltaSeconds :type Float%20%28single-precision%29)))

(fn ConstructionScript)