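; StreetNodeData is a pathfinding actor for the AI traffic system that gathers every FixedStreetNode at BeginPlay.
; GetShortestPath runs Dijkstra over NextNodes links, storing Distance and Previous on each node, then returns the path ordered target to start.
; Each step's cost is measured from this actor's own location to the neighbour, not from the current node.
; DrawShortestPath highlights the result by switching each path node's AcceptSphere to its active material.
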(event Custom|DrawShortestPath
  ;[1 1 1] Get all Nodes from the Shortest patch and switch their Material from inactive to active
  (for _array_element (Variables|Default|GetShortestPath)
    (Rendering|Material|SetMaterial (Variables|/Game/VRDrivingSimulator/AI/AIVehicle/TrafficSystem/Blueprints/FixedStreetNode.FixedStreetNode_C|GetAcceptSphere _array_element) 0 (Variables|/Game/VRDrivingSimulator/AI/AIVehicle/TrafficSystem/Blueprints/FixedStreetNode.FixedStreetNode_C|GetActiveMat _array_element))))

(event EventBeginPlay
  ;[1 1 1] Gather all StreetNodes!
  (bind _outactors (Actor|GetAllActorsOfClass "/Game/VRDrivingSimulator/AI/AIVehicle/TrafficSystem/Blueprints/FixedStreetNode.FixedStreetNode_C"))
  (Variables|Default|SetAllNodes _outactors))

(fn ConstructionScript)

(fn GetShortestPath
  (params (StartNode :type Fixed%20Street%20Node%20Object%20Reference) (TargetNode :type Fixed%20Street%20Node%20Object%20Reference))
  ;[1 1 1] Clear our latest shortest path
  (Utilities|Array|Clear (Variables|Default|GetShortestPath))
  ;[1 1 1] Initialize variables for the Dijkstra Algorithm
  (Variables|Default|SetStartNodeRef StartNode)
  (Variables|/Game/VRDrivingSimulator/AI/AIVehicle/TrafficSystem/Blueprints/FixedStreetNode.FixedStreetNode_C|SetDistance StartNode 0.0)
  (Variables|/Game/VRDrivingSimulator/AI/AIVehicle/TrafficSystem/Blueprints/FixedStreetNode.FixedStreetNode_C|SetPrevious StartNode 0)
  (Variables|Default|SetTargetNodeRef TargetNode)
  (for _array_element (Variables|Default|GetAllNodes)
    (Utilities|Array|Add (Variables|Default|GetUnvisited) _array_element)
    (if (!= _array_element StartNode)
      (Variables|/Game/VRDrivingSimulator/AI/AIVehicle/TrafficSystem/Blueprints/FixedStreetNode.FixedStreetNode_C|SetDistance _array_element 1e+10)
      (Variables|/Game/VRDrivingSimulator/AI/AIVehicle/TrafficSystem/Blueprints/FixedStreetNode.FixedStreetNode_C|SetPrevious _array_element 0)))
  (Development|PrintString "Completed Init" false)
  (Variables|Default|SetBreakWhile true)
  (while (and (> (Utilities|Array|Length (Variables|Default|GetUnvisited)) 0) (Variables|Default|GetBreakWhile))
    (Variables|Default|SetMinDistance 1e+08)
    (Variables|Default|SetCurrentNode 0)
    (for _array_element_2 (Variables|Default|GetUnvisited)
      ;[1 1 1] Get the node that has the minimum distance
      (if (< (Variables|/Game/VRDrivingSimulator/AI/AIVehicle/TrafficSystem/Blueprints/FixedStreetNode.FixedStreetNode_C|GetDistance _array_element_2) (Variables|Default|GetMinDistance))
        (Variables|Default|SetCurrentNode _array_element_2)
        (Variables|Default|SetMinDistance (Variables|/Game/VRDrivingSimulator/AI/AIVehicle/TrafficSystem/Blueprints/FixedStreetNode.FixedStreetNode_C|GetDistance _array_element_2))))
    (Development|PrintString "Completed minDist Node" false)
    (Utilities|IsValid (Variables|Default|GetCurrentNode)
      (:Is%20Valid
        ;[1 1 1] Check if we are not looking at the TargetNode
        (if (!= (Variables|Default|GetCurrentNode) (Variables|Default|GetTargetNodeRef))
          (Utilities|Array|RemoveItem (Variables|Default|GetUnvisited) (Variables|Default|GetCurrentNode))
          ;[1 1 1] Check if the new Distance coming with this Path is shorter and update the Node
          (for _array_element_3 (Variables|/Game/VRDrivingSimulator/AI/AIVehicle/TrafficSystem/Blueprints/FixedStreetNode.FixedStreetNode_C|GetNextNodes (Variables|Default|GetCurrentNode))
            (if (Utilities|Array|ContainsItem (Variables|Default|GetUnvisited) _array_element_3)
              (bind _output_get (Variables|Default|SetTempDistance (+ (Variables|/Game/VRDrivingSimulator/AI/AIVehicle/TrafficSystem/Blueprints/FixedStreetNode.FixedStreetNode_C|GetDistance (Variables|Default|GetCurrentNode)) (Math|Vector|VectorLength (- (Transformation|GetActorLocation) (Transformation|GetActorLocation _array_element_3))))))
              (if (< _output_get (Variables|/Game/VRDrivingSimulator/AI/AIVehicle/TrafficSystem/Blueprints/FixedStreetNode.FixedStreetNode_C|GetDistance _array_element_3))
                (Variables|/Game/VRDrivingSimulator/AI/AIVehicle/TrafficSystem/Blueprints/FixedStreetNode.FixedStreetNode_C|SetDistance _array_element_3 _output_get)
                (Variables|/Game/VRDrivingSimulator/AI/AIVehicle/TrafficSystem/Blueprints/FixedStreetNode.FixedStreetNode_C|SetPrevious _array_element_3 (Variables|Default|GetCurrentNode)))))
          (Development|PrintString "Checked all NextNodes" false)
          (else
            (Variables|Default|SetBreakWhile false :!label _label))))
      (:Is%20Not%20Valid
        (Development|PrintString "CurrentNode is NULL")
        (goto _label))))
  (Development|PrintString "Completed While" false)
  ;[1 1 1] Now, that we got the shortest path. We take the last Node (TargetNode) and just go from back to front through all the "Previous" nodes and add them to the shortest path array
  (bind _output_get_2 (Variables|Default|SetTempNode (Variables|Default|GetTargetNodeRef)))
  (if (!= _output_get_2 (Variables|Default|GetStartNodeRef))
    (while (!= (Variables|/Game/VRDrivingSimulator/AI/AIVehicle/TrafficSystem/Blueprints/FixedStreetNode.FixedStreetNode_C|GetPrevious (Variables|Default|GetTempNode)) 0)
      (Utilities|Array|Add (Variables|Default|GetShortestPath) (Variables|Default|GetTempNode))
      (Variables|Default|SetTempNode (Variables|/Game/VRDrivingSimulator/AI/AIVehicle/TrafficSystem/Blueprints/FixedStreetNode.FixedStreetNode_C|GetPrevious (Variables|Default|GetTempNode))))
    (else
      (Development|PrintString "Start is Alread the End" false)))
  (Utilities|Array|Add (Variables|Default|GetShortestPath) (Variables|Default|GetStartNodeRef))
  (Development|PrintString "ShortestPath found")
  (return (Variables|Default|GetShortestPath)))