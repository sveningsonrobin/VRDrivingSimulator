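; Dashboard speedometer Blueprint that shows the player vehicle's current speed on an analog needle and a text readout.
; Each tick it casts the player pawn to WheeledVehicle and converts the absolute forward speed from units per second to km/h.
; That value drives the Arrow component's yaw as a linear offset from a resting angle and sets the TextRender to the truncated whole number.
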(event EventTick
  (params (DeltaSeconds :type Float%20%28single-precision%29))
  (bind _aswheeled_vehicle (Utilities|Casting|CastToWheeledVehicle (Game|Player|GetPlayerPawn 0)))
  (Transformation|SetRelativeRotation (Variables|Default|GetArrow) (Math|Rotator|MakeRotator 0.0 0.0 (+ -135.0 (* 2.2 (Math|Float|Absolute(Float) (* (Vehicle|GetForwardSpeed (Variables|/Script/Engine.WheeledVehicle|GetVehicleMovement _aswheeled_vehicle)) 0.036))))) false false)
  (Rendering|Components|TextRender|SetText (Variables|Default|GetTextRender) (Utilities|Text|ToText(String) (Utilities|String|BuildString(Integer) "" "" (Math|Float|Truncate (Math|Float|Absolute(Float) (* (Vehicle|GetForwardSpeed (Variables|/Script/Engine.WheeledVehicle|GetVehicleMovement _aswheeled_vehicle)) 0.036)))))))

(fn ConstructionScript)