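; Street light actor for the VR driving simulator whose lamp switches between lit and unlit looks.
; Tick compares the ONOFF flag with LASTONOFF and acts only when they differ, swapping the Lamp's first material between the ON and OFF versions.
; It then updates LASTONOFF; nothing in this graph sets ONOFF or changes a light component.
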(event EventActorBeginOverlap
  (params (OtherActor :type Actor%20Object%20Reference)))

(event EventTick
  (params (DeltaSeconds :type Float%20%28single-precision%29))
  (bind _on_off (Variables|Default|GetON/OFF))
  (if (Class|KismetMathLibrary|XORBoolean _on_off (Variables|Default|GetLAST_ON/OFF))
    (if _on_off
      (Rendering|Material|SetMaterial (Variables|Default|GetLamp) 0 "/Game/VRDrivingSimulator/Materials/Street_light_ON.Street_light_ON")
      (Variables|Default|SetLAST_ON/OFF true)
      (else
        (Rendering|Material|SetMaterial (Variables|Default|GetLamp) 0 "/Game/VRDrivingSimulator/Materials/Street_light_OFF.Street_light_OFF")
        (Variables|Default|SetLAST_ON/OFF false)))))

(event EventBeginPlay)

(fn ConstructionScript)